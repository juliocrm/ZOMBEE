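; BP_AttackComp is an attack component that deals delayed area damage to actors on other teams.
; Attack raises OnAttack and starts a timer at 65% of AttackTime, blocking re-entry while Attacking.
; The delayed hit scans OverlapSphere and applies negative stamina through each opposing actor's BP_HealthBaseComp, passing hit direction and owner as perpetrator.
; The Dead event clears CanAttack, which blocks new attacks and any pending hit.
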(event EventBeginPlay)

(event EventTick
  (params (DeltaSeconds :type Float%20%28single-precision%29)))

(event EventDead
  (Variables|Default|SetCanAttack false))

(fn Attack
  (if (not (Variables|Default|GetAttacking))
    (if (Variables|Default|GetCanAttack)
      (Variables|Default|SetAttacking true)
      (Default|CallOnAttack self)
      (Utilities|Time|SetTimerbyEvent (EventDispatchers|CreateEvent :!event AfterDelayAttack) (* (Variables|Default|GetAttackTime) 0.65)))))

(fn AfterDelayAttack
  (bind _returnvalue (Components|GetOwner))
  (if (Variables|Default|GetCanAttack)
    (Variables|Default|SetAttacking false)
    (for _array_element (Collision|GetOverlappingActors (Variables|Default|GetOverlapSphere) 0 :!class /Script/Engine.PrimitiveComponent)
      (Utilities|IsValid (Actor|GetComponentbyClass _array_element "/Game/GGJ2019/Models/Bee/BP_TeamComp.BP_TeamComp_C")
        (:Is%20Valid
          (if (!= (Variables|/Game/GGJ2019/Models/Bee/BP_TeamComp.BP_TeamComp_C|GetTeam (Actor|GetComponentbyClass (Components|GetOwner) "/Game/GGJ2019/Models/Bee/BP_TeamComp.BP_TeamComp_C")) (Variables|/Game/GGJ2019/Models/Bee/BP_TeamComp.BP_TeamComp_C|GetTeam (Actor|GetComponentbyClass _array_element "/Game/GGJ2019/Models/Bee/BP_TeamComp.BP_TeamComp_C")))
            (Default|AddStamina (Actor|GetComponentbyClass _array_element "/Game/GGJ2019/Models/Bee/BP_HealthBaseComp.BP_HealthBaseComp_C") (* (Variables|Default|GetDamage) -1.0) true (Math|Vector|Normalize (- (Transformation|GetActorLocation _array_element) (Transformation|GetActorLocation _returnvalue))) _returnvalue)))))))