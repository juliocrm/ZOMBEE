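; Health component for an actor that tracks damage and death and spawns blood effects.
; AddStamina clamps CurrentHealth, fires Hurted on external non-positive changes, or at zero sends DeadMessage to all owner components and calls Dead.
; Its own Hurted and Dead handlers spawn BloodSystem rotated along the perpetrator-to-owner direction, for deaths only when external.
; Tick draws debug health text above living owners below or otherwise off max health.
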(event Custom|Hurted_Event
  (params (EventTarget :type BP%20Health%20Base%20Comp%20Object%20Reference) (Amount :type Float%20%28single-precision%29) (DamageDirection :type Vector) (Perpetrator :type Actor%20Object%20Reference))
  (bind _returnvalue (Components|GetOwner))
  (bind _returnvalue_2 (Transformation|GetActorLocation _returnvalue))
  (Niagara|SpawnSystematLocation (Variables|Default|GetBloodSystem) _returnvalue_2 (Math|Rotator|FindLookatRotation (Transformation|GetActorLocation Perpetrator) _returnvalue_2)))

(event Custom|Dead_Event_0
  (params (EventTarget :type BP%20Health%20Base%20Comp%20Object%20Reference) (LastDamage :type Float%20%28single-precision%29) (IsExternal :type Boolean) (DamageDirection :type Vector) (Perpetrator :type Actor%20Object%20Reference))
  (if IsExternal
    (Niagara|SpawnSystematLocation (Variables|Default|GetBloodSystem) "0, 0, 0" (Math|Rotator|FindLookatRotation (Transformation|GetActorLocation Perpetrator) (Transformation|GetActorLocation (Components|GetOwner))))))

(event EventBeginPlay
  (EventDispatchers|BindEventtoHurted (delegate Custom|Hurted_Event))
  (EventDispatchers|AssignDead (delegate Custom|Dead_Event_0)))

(event EventTick
  (params (DeltaSeconds :type Float%20%28single-precision%29))
  (bind _currenthealth (Variables|Default|GetCurrentHealth))
  (bind _maxhealth (Variables|Default|GetMaxHealth))
  (if (and (!= _currenthealth _maxhealth) (> _currenthealth 0.0))
    (Rendering|Debug|DrawDebugString (+ (Transformation|GetActorLocation (Components|GetOwner)) "0, 0,200.000000") (Utilities|String|Append (Utilities|String|ToString(Float) _currenthealth) "/" (Utilities|String|ToString(Float) _maxhealth)) 0 "(R=0.426639,G=1.000000,B=0.320916,A=1.000000)")))

(fn AddStamina
  (params (Amount :type Float%20%28single-precision%29) (IsExternal :type Boolean) (DamageDirection :type Vector) (Perpetrator :type Actor%20Object%20Reference))
  (Utilities|FlowControl|Sequence
    (:then_0
      (Variables|Default|SetCurrentHealth (Math|Float|Clamp(Float) (+ (Variables|Default|GetCurrentHealth) Amount) 0.0 (Variables|Default|GetMaxHealth))))
    (:then_1
      (if (> (Variables|Default|GetCurrentHealth) 0.0)
        (if (not (> Amount 0.0))
          (if IsExternal
            (Niagara|SpawnSystemAttached 0 0 "None" "0, 0, 0" "0, 0, 0" "KeepRelativeOffset" false)
            (Default|CallHurted self Amount DamageDirection Perpetrator)))
        (else
          (Utilities|FlowControl|Sequence
            (:then_0
              (for _array_element (Actor|GetComponentsByClass (Components|GetOwner) "/Script/Engine.ActorComponent")
                (Class|ICanDie|Dead(Message) _array_element)))
            (:then_1
              (Default|CallDead self Amount IsExternal DamageDirection Perpetrator))))))))