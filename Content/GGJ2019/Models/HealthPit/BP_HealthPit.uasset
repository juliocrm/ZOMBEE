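; BP_HealthPit is a healing pit with a finite honey reserve that restores an overlapping actor's health over time.
; Box overlap latches one BP_HealthBaseComp at a time, released when its owner leaves.
; Tick calls AddStamina on it, capped by missing health, heal rate and remaining reserve, and toggles Niagara spawning.
; The honey mesh lerps toward the Rer component's transform as the reserve drains, hiding when empty.
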(event OnComponentBeginOverlap(Box)
  (params (OverlappedComponent :type Primitive%20Component%20Object%20Reference) (OtherActor :type Actor%20Object%20Reference) (OtherComp :type Primitive%20Component%20Object%20Reference) (OtherBodyIndex :type Integer) (bFromSweep :type Boolean) (SweepResult :type Hit%20Result%20Structure%20%28by%20ref%29))
  (Variables|Default|GetHealReceptor
    (:then)
    (:else
      (Variables|Default|SetHealReceptor (Actor|GetComponentbyClass OtherActor "/Game/GGJ2019/Models/Bee/BP_HealthBaseComp.BP_HealthBaseComp_C")))))

(event OnComponentEndOverlap(Box)
  (params (OverlappedComponent :type Primitive%20Component%20Object%20Reference) (OtherActor :type Actor%20Object%20Reference) (OtherComp :type Primitive%20Component%20Object%20Reference) (OtherBodyIndex :type Integer))
  (bind _healreceptor (Variables|Default|GetHealReceptor)
    (:then
      (if (== (Actor|GetComponentbyClass OtherActor "/Game/GGJ2019/Models/Bee/BP_HealthBaseComp.BP_HealthBaseComp_C") _healreceptor)
        (Variables|Default|SetHealReceptor 0)))
    (:else)))

(event EventBeginPlay
  (bind _niagara (Variables|Default|GetNiagara))
  (Variables|Default|SetLifeToHeal (Variables|Default|GetMaxLifeToHeal))
  (Variables|Default|SetInitialHoneyTransform (Transformation|GetRelativeTransform (Variables|Default|GetSM_Life_Honney)))
  (Rendering|SetVisibility _niagara true false)
  (Niagara|SetNiagaraVariable(Float) _niagara "User.SpawnRate" 0.0))

(event Collision|EventActorBeginOverlap
  (params (OtherActor :type Actor%20Object%20Reference)))

(event EventTick
  (params (DeltaSeconds :type Float%20%28single-precision%29))
  (bind _healreceptor (Variables|Default|GetHealReceptor)
    (:then
      (if (> (- (Variables|/Game/GGJ2019/Models/Bee/BP_HealthBaseComp.BP_HealthBaseComp_C|GetMaxHealth _healreceptor) (Variables|/Game/GGJ2019/Models/Bee/BP_HealthBaseComp.BP_HealthBaseComp_C|GetCurrentHealth _healreceptor)) 0.0)
        (Niagara|SetNiagaraVariable(Float) (Variables|Default|GetNiagara) "User.SpawnRate" 1.0)
        (Default|AddStamina _healreceptor (Math|Float|Min(Float) (- (Variables|/Game/GGJ2019/Models/Bee/BP_HealthBaseComp.BP_HealthBaseComp_C|GetMaxHealth _healreceptor) (Variables|/Game/GGJ2019/Models/Bee/BP_HealthBaseComp.BP_HealthBaseComp_C|GetCurrentHealth _healreceptor)) (* DeltaSeconds (Variables|Default|GetHealPerSec)) (Variables|Default|GetLifeToHeal)) false "0, 0, 0")
        (Variables|Default|SetLifeToHeal (- (Variables|Default|GetLifeToHeal) (Math|Float|Min(Float) (- (Variables|/Game/GGJ2019/Models/Bee/BP_HealthBaseComp.BP_HealthBaseComp_C|GetMaxHealth _healreceptor) (Variables|/Game/GGJ2019/Models/Bee/BP_HealthBaseComp.BP_HealthBaseComp_C|GetCurrentHealth _healreceptor)) (* DeltaSeconds (Variables|Default|GetHealPerSec)) (Variables|Default|GetLifeToHeal))))
        (if (<= (Variables|Default|GetLifeToHeal) 0.0)
          (Rendering|SetVisibility (Variables|Default|GetSM_Life_Honney) false true)
          (else
            (Rendering|SetVisibility (Variables|Default|GetSM_Life_Honney) true true)
            (Transformation|SetRelativeTransform (Variables|Default|GetSM_Life_Honney) (Math|Transform|Lerp(Transform) (Transformation|GetRelativeTransform (Variables|Default|Getrer)) (Variables|Default|GetInitialHoneyTransform) (/ (Variables|Default|GetLifeToHeal) (Variables|Default|GetMaxLifeToHeal))) false true)))
        (else
          (Niagara|SetNiagaraVariable(Float) (Variables|Default|GetNiagara) "User.SpawnRate" 0.0 :!label _label))))
    (:else
      (goto _label))))

(fn ConstructionScript)